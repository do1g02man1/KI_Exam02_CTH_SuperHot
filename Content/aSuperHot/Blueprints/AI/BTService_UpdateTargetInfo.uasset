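; Behavior tree service for the AI that tracks the player pawn as a target and writes what it finds to the blackboard.
; Each tick it stores the distance to the player, then runs a Visibility line trace from the controlled pawn to the player.
; A clear hit sets the target actor and clears the wall flag; otherwise only the flag is raised, leaving any previous target in place.
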(event `self.ReceiveTickAI`
  (params (OwnerController :type "AIController Object Reference") (ControlledPawn :type "Pawn Object Reference") (DeltaSeconds :type "Float (single-precision)"))
  (bind _returnvalue (`Actor.K2_GetActorLocation` ControlledPawn))
  (bind _returnvalue_2 (`GameplayStatics.GetPlayerPawn` 0))
  (bind _returnvalue_3 (`Actor.K2_GetActorLocation` (`GameplayStatics.GetPlayerPawn` 0)))
  (`/Engine/EditorBlueprintResources/StandardMacros.IsValid` (`GameplayStatics.GetPlayerPawn` 0)
    (:`Is Valid`
      (`BTFunctionLibrary.SetBlackboardValueAsFloat` (`self.TargetDistanceKey`) (`KismetMathLibrary.VSize` (- _returnvalue _returnvalue_3)))
      (bind _outhit (`KismetSystemLibrary.LineTraceSingle` :`Start` _returnvalue :`End` _returnvalue_3 :`TraceChannel` "TraceTypeQuery1" :`DrawTime` 1.0))
      (if (== (`.HitActor` (`GameplayStatics.BreakHitResult` _outhit)) _returnvalue_2)
        (`BTFunctionLibrary.SetBlackboardValueAsObject` (`self.TargetActorKey`) _returnvalue_2)
        (`BTFunctionLibrary.SetBlackboardValueAsBool` (`self.IsBetweenWallKey`))
        (else
          (`BTFunctionLibrary.SetBlackboardValueAsBool` (`self.IsBetweenWallKey`) true))))))