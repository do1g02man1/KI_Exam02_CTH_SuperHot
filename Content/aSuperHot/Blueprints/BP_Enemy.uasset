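; BP_Enemy is an AI-controlled pistol enemy that shoots at the player and shatters when killed.
; A hit from a player-owned actor stops its AI logic, disables collision and plays a death montage.
; At the montage notify, it swaps itself for BP_GC_Enemy and triggers an FS_MasterField to break it apart.
; EnemyShoot spawns a projectile from the pistol socket on a montage notify, with velocity aimed straight at the player.
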(event `self.ReceiveHit`
  (params (MyComp :type "PrimitiveComponent Object Reference") (Other :type "Actor Object Reference") (OtherComp :type "PrimitiveComponent Object Reference") (bSelfMoved :type Boolean) (HitLocation :type "Vector Structure") (HitNormal :type "Vector Structure") (NormalImpulse :type "Vector Structure") (Hit :type "HitResult Structure (by ref)"))
  (bind _diedlocation (`self.DiedLocation`))
  (if (== (`self.GetOwner` Other) (`GameplayStatics.GetPlayerPawn` 0))
    (bind _asbp_enemy_aicontroller (cast `/Game/aSuperHot/Blueprints/AI/BP_EnemyAIController` (`self.GetController`)))
    (`BrainComponent.StopLogic` (`AIController.BrainComponent` _asbp_enemy_aicontroller) "Dead")
    (`PrimitiveComponent.SetCollisionEnabled` (`self.CapsuleComponent`) "NoCollision")
    (`PrimitiveComponent.SetCollisionEnabled` (`self.Mesh`) "NoCollision")
    (`|PlayMontage` (`self.Mesh`) "/Game/aSuperHot/Animation/AM_Dead.AM_Dead" 1.0 0.0 "EnemyTest"
      (:`then`
        (set `self.DiedLocation` (`self.GetTransform`)))
      (:`OnNotifyBegin`
        (`self.K2_DestroyActor`)
        (`|SpawnActorFromClass` "/Game/aSuperHot/Blueprints/BP_GC_Enemy.BP_GC_Enemy_C" (`KismetMathLibrary.MakeTransform` (+ (.location _diedlocation) (0.0 0.0 -100.0)) (`KismetMathLibrary.MakeRotator` (.roll (.rotation _diedlocation)) (.pitch (.rotation _diedlocation)) (+ (.yaw (.rotation _diedlocation)) -90.0)) (.scale _diedlocation)) "Undefined" "MultiplyWithRoot" null null)
        (bind _returnvalue (`|SpawnActorFromClass` "/Engine/EditorResources/FieldNodes/FS_MasterField.FS_MasterField_C" (`self.DiedLocation`) "Undefined" "MultiplyWithRoot" null null))
        (set `/Engine/EditorResources/FieldNodes/FS_MasterField.ActivationType` "NewEnumerator4" _returnvalue)
        (`/Engine/EditorResources/FieldNodes/FS_MasterField.CE_Trigger` _returnvalue)))))

(event `EnemyShoot`
  (bind _returnvalue (`KismetMathLibrary.RandomFloatInRange` -20.0 -20.0))
  (bind _returnvalue_2 (`SceneComponent.GetSocketLocation` (`self.Pistol`) "EnemyAmmo"))
  (bind _returnvalue_3 (`KismetMathLibrary.Normal` (- (`self.K2_GetActorLocation` (`GameplayStatics.GetPlayerCharacter` 0)) _returnvalue_2)))
  (bind (_returnvalue_roll _returnvalue_pitch _returnvalue_yaw) (`KismetMathLibrary.BreakRotator` (`KismetMathLibrary.MakeRotFromX` _returnvalue_3)))
  (`|PlayMontage` (`self.Mesh`) "/Game/aSuperHot/Animation/AM_EnemyFiringPistol.AM_EnemyFiringPistol" 1.0 0.0 "Fire"
    (:`OnNotifyBegin`
      (bind _returnvalue_4 (`|SpawnActorFromClass` "/Game/aSuperHot/Blueprints/Projectile/BP_EnemyBulletProjectile.BP_EnemyBulletProjectile_C" (`KismetMathLibrary.MakeTransform` _returnvalue_2 (`KismetMathLibrary.MakeRotator` (+ _returnvalue_roll _returnvalue) (+ _returnvalue_pitch _returnvalue) (+ _returnvalue_yaw _returnvalue))) "Undefined" "MultiplyWithRoot" (`self.GetOwner`) null))
      (bind _projectilemovement (`/Game/aSuperHot/Blueprints/Projectile/BP_EnemyBulletProjectile.ProjectileMovement` _returnvalue_4))
      (set `MovementComponent.Velocity` (* _returnvalue_3 (`ProjectileMovementComponent.MaxSpeed` _projectilemovement)) _projectilemovement))))

(fn `UserConstructionScript`)