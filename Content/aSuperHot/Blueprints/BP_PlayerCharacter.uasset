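; First-person player character for a SUPERHOT-style game, where global time dilation follows the player's input.
; Looking slows time and moving restores full speed; releasing either returns to the GameInstance's baseline value while alive.
; It also adds the crosshair and Enhanced Input mapping, and can detach and destroy the current weapon.
; Death runs once, removing input, restoring time, fading to white and reloading the level; jump is unwired.
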(event `self.ReceiveBeginPlay`
  (bind _asbp_time_dilation_variable (cast `/Game/aSuperHot/Blueprints/BP_TimeDilationVariable` (`GameplayStatics.GetGameInstance`)))
  (bind _output_get (set `self.TimeDilationVariable` _asbp_time_dilation_variable))
  (`GameplayStatics.SetGlobalTimeDilation` (`/Game/aSuperHot/Blueprints/BP_TimeDilationVariable.TimeDilationControl` _output_get))
  (bind _returnvalue (`|CreateWidget` "/Game/aSuperHot/UI/WBP_Crosshair.WBP_Crosshair_C" (`GameplayStatics.GetPlayerController` 0)))
  (`UserWidget.AddToViewport` _returnvalue 0))

(event `self.ReceiveControllerChanged`
  (params (OldController :type "Controller Object Reference") (NewController :type "Controller Object Reference"))
  (bind `_as플레이어_컨트롤러` (cast `PlayerController` NewController))
  (bind _output_get (set `self.PlayerController` `_as플레이어_컨트롤러`))
  (`EnhancedInputSubsystemInterface.AddMappingContext` (pcsubsystem `EnhancedInputLocalPlayerSubsystem` _output_get) "/Game/aSuperHot/Input/IMC_Default.IMC_Default" 0 (struct)))

(event `EnhancedInput|/Game/aSuperHot/Input/Actions/IA_Look`
  (params (ActionValue :type "Vector2D Structure") (ElapsedSeconds :type "Float (double-precision)") (TriggeredSeconds :type "Float (double-precision)") (InputAction :type "InputAction Object Reference" :default "/Game/aSuperHot/Input/Actions/IA_Look.IA_Look"))
  (:`Triggered`
    (`self.AddControllerYawInput` ActionValue_X)
    (`self.AddControllerPitchInput` ActionValue_Y)
    (`GameplayStatics.SetGlobalTimeDilation` 0.3 :!label _label))
  (:`Started`
    (goto _label))
  (:`Completed`
    (if (not (`self.IsDead`))
      (`GameplayStatics.SetGlobalTimeDilation` (`/Game/aSuperHot/Blueprints/BP_TimeDilationVariable.TimeDilationControl` (`self.TimeDilationVariable`))))))

(event `EnhancedInput|/Game/aSuperHot/Input/Actions/IA_Move`
  (params (ActionValue :type "Vector2D Structure") (ElapsedSeconds :type "Float (double-precision)") (TriggeredSeconds :type "Float (double-precision)") (InputAction :type "InputAction Object Reference" :default "/Game/aSuperHot/Input/Actions/IA_Move.IA_Move"))
  (:`Triggered`
    (`self.AddMovementInput` (`self.GetActorRightVector`) ActionValue_X)
    (`self.AddMovementInput` (`self.GetActorForwardVector`) ActionValue_Y)
    (`GameplayStatics.SetGlobalTimeDilation` 1.0)
    (`CameraComponent.SetPostProcessBlendWeight` (`self.FirstPersonCamera`) 1.0))
  (:`Completed`
    (if (not (`self.IsDead`))
      (`GameplayStatics.SetGlobalTimeDilation` (`/Game/aSuperHot/Blueprints/BP_TimeDilationVariable.TimeDilationControl` (`self.TimeDilationVariable`))))))

(event `EnhancedInput|/Game/aSuperHot/Input/Actions/IA_Jump`
  (params (ActionValue :type Boolean) (ElapsedSeconds :type "Float (double-precision)") (TriggeredSeconds :type "Float (double-precision)") (InputAction :type "InputAction Object Reference" :default "/Game/aSuperHot/Input/Actions/IA_Jump.IA_Jump")))

(event `IsEquipWeapon`
  (bind _currentweapon (`self.CurrentWeapon`))
  (if (!= null (`self.CurrentWeapon`))
    (`SceneComponent.K2_DetachFromComponent` _currentweapon "KeepWorld" "KeepWorld" "KeepWorld" true)
    (`ActorComponent.K2_DestroyComponent` _currentweapon)
    (set `self.CurrentWeapon` null)
    (set `self.WeaponType` "NewEnumerator0")))

(event `Dead`
  (bind _returnvalue (pcsubsystem `EnhancedInputLocalPlayerSubsystem` (`self.PlayerController`)))
  (`/Engine/EditorBlueprintResources/StandardMacros.DoOnce` false ; 한번만 실행하기
    (:`Completed`
      (set `self.IsDead` true)
      (`EnhancedInputSubsystemInterface.RemoveMappingContext` _returnvalue "/Game/aSuperHot/Input/IMC_Default.IMC_Default" (struct))
      (`EnhancedInputSubsystemInterface.RemoveMappingContext` _returnvalue "/Game/aSuperHot/Input/IMC_Weapons.IMC_Weapons" (struct))
      (`KismetSystemLibrary.Delay` 0.01)
      (`GameplayStatics.SetGlobalTimeDilation` 1.0)
      (`PlayerCameraManager.StartCameraFade` (`GameplayStatics.GetPlayerCameraManager` 0) 0.0 1.0 1.0 (struct :`R` 1.0 :`G` 1.0 :`B` 1.0 :`A` 1.0) false true)
      (`KismetSystemLibrary.Delay` 2.0)
      (bind _returnvalue_2 (`GameplayStatics.GetCurrentLevelName` true))
      (`GameplayStatics.OpenLevel` (`KismetStringLibrary.Conv_StringToName` _returnvalue_2)))))

(fn `UserConstructionScript`)