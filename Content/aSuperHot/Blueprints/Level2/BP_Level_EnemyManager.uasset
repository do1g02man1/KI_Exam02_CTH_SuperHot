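; Level enemy manager that advances the game to the next level once all enemies are dead.
; BeginPlay counts the placed BP_LevelEnemy actors, and OnEnemyDied decrements that count.
; At zero, after a short delay, it checks the current level name to open Level2 from Level1 or Level3 from Level2, and quits the game from any other level.
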(event `self.ReceiveBeginPlay`
  (bind _outactors (`GameplayStatics.GetAllActorsOfClass` "/Game/aSuperHot/Blueprints/Level2/BP_LevelEnemy.BP_LevelEnemy_C"))
  (set `self.EnemyCount` (`KismetArrayLibrary.Array_Length` _outactors)))

(event `OnEnemyDied`
  (bind _output_get (set `self.EnemyCount` (- (`self.EnemyCount`) 1)))
  (if (== _output_get 0)
    (`KismetSystemLibrary.Delay` 3.0)
    (bind _returnvalue (`GameplayStatics.GetCurrentLevelName` true))
    (bind _returnvalue_2 (`KismetStringLibrary.Conv_StringToName` _returnvalue))
    (if (== _returnvalue_2 "Level1")
      (`GameplayStatics.OpenLevel` "Level2")
      (elif (== _returnvalue_2 "Level2")
        (`GameplayStatics.OpenLevel` "Level3")
        (else
          (`KismetSystemLibrary.QuitGame` null "Quit"))))))

(fn `UserConstructionScript`)