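; Bullet projectile actor for the SuperHot-style game that sets off a physics field where it hits.
; On hit, it spawns an FS_MasterField at the impact location, sets its activation type and triggers it, then destroys itself after a short delay.
; Tick and BeginPlay do nothing, leaving disconnected experiments for Niagara trail time and an owner-name debug print.
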(event `self.ReceiveTick`
  (params (DeltaSeconds :type "Float (single-precision)"))
  ; 나이아가라 파티클 시간 흐름 영향 안 받게
  ; (필요없음)
)

(event `self.ReceiveBeginPlay`
  ; 총알의 Owner 체크 ( 적 피격 시 판단하기 위해서 )
)

(event `self.ReceiveHit`
  (params (MyComp :type "PrimitiveComponent Object Reference") (Other :type "Actor Object Reference") (OtherComp :type "PrimitiveComponent Object Reference") (bSelfMoved :type Boolean) (HitLocation :type "Vector Structure") (HitNormal :type "Vector Structure") (NormalImpulse :type "Vector Structure") (Hit :type "HitResult Structure (by ref)"))
  (bind _returnvalue (`|SpawnActorFromClass` "/Engine/EditorResources/FieldNodes/FS_MasterField.FS_MasterField_C" (`KismetMathLibrary.MakeTransform` HitLocation) "Undefined" "MultiplyWithRoot" null null))
  (set `/Engine/EditorResources/FieldNodes/FS_MasterField.ActivationType` "NewEnumerator4" _returnvalue)
  (`/Engine/EditorResources/FieldNodes/FS_MasterField.CE_Trigger` _returnvalue)
  (`KismetSystemLibrary.Delay` 0.2)
  (`self.K2_DestroyActor`))

(fn `UserConstructionScript`)