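; Rifle weapon component that attaches to the player's first-person mesh at the grip socket, enables weapon input and sets the player's weapon type.
; Shooting spawns a camera-aimed bullet, plays the firing montage and briefly pulses global time dilation before restoring the GameInstance's value.
; Throwing spawns the rifle as a projectile and calls the player's equip-weapon function.
; Each action alerts all enemy AI controllers only on first use, via DoOnce.
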(event `self.ReceiveBeginPlay`
  (bind _asbp_time_dilation_variable (cast `/Game/aSuperHot/Blueprints/BP_TimeDilationVariable` (`GameplayStatics.GetGameInstance`)))
  (set `self.TimeDilationVariable` _asbp_time_dilation_variable)
  (bind _asbp_player_character (cast `/Game/aSuperHot/Blueprints/BP_PlayerCharacter` (`self.GetOwner`)))
  (set `self.First PersonCharacter` _asbp_player_character)
  (bind _firstpersonmesh (`/Game/aSuperHot/Blueprints/BP_PlayerCharacter.FirstPersonMesh` _asbp_player_character))
  (`/Engine/EditorBlueprintResources/StandardMacros.IsValid` (`self.GetAttachParent` _firstpersonmesh)
    (:`Is Valid`
      (if (== "RifleGripPoint" (`Actor.GetAttachParentSocketName` (`self.First PersonCharacter`)))
        (`self.K2_DetachFromComponent` _firstpersonmesh "KeepRelative" "KeepRelative" "KeepRelative" true))
      (`self.K2_AttachToComponent` _firstpersonmesh "RifleGripPoint" "SnapToTarget" "SnapToTarget" "SnapToTarget")
      (bind `_as플레이어_컨트롤러` (cast `PlayerController` (`Pawn.GetController` (`self.First PersonCharacter`))))
      (bind _returnvalue (pcsubsystem `EnhancedInputLocalPlayerSubsystem` `_as플레이어_컨트롤러`))
      (`/Engine/EditorBlueprintResources/StandardMacros.IsValid` _returnvalue
        (:`Is Valid`
          (`EnhancedInputSubsystemInterface.AddMappingContext` _returnvalue "/Game/aSuperHot/Input/IMC_Weapons.IMC_Weapons" 1 (struct))
          (bind _asbp_player_character_2 (cast `/Game/aSuperHot/Blueprints/BP_PlayerCharacter` (`self.GetOwner`)))
          (set `/Game/aSuperHot/Blueprints/BP_PlayerCharacter.WeaponType` "NewEnumerator2" _asbp_player_character_2))))))

(event `EnhancedInput|/Game/aSuperHot/Input/Actions/IA_Shoot`
  (params (ActionValue :type Boolean) (ElapsedSeconds :type "Float (double-precision)") (TriggeredSeconds :type "Float (double-precision)") (InputAction :type "InputAction Object Reference" :default "/Game/aSuperHot/Input/Actions/IA_Shoot.IA_Shoot"))
  (bind _returnvalue (`PlayerCameraManager.GetCameraRotation` (`GameplayStatics.GetPlayerCameraManager` 0)))
  (:`Triggered`
    (`|SpawnActorFromClass` "/Game/aSuperHot/Blueprints/Projectile/BP_BulletProjectile.BP_BulletProjectile_C" (`KismetMathLibrary.MakeTransform` (+ (`self.GetSocketLocation` "Ammo") (`KismetMathLibrary.GreaterGreater_VectorRotator` (`self.ProjectileOffset`) _returnvalue)) _returnvalue) "Undefined" "OverrideRootScale" (`self.GetOwner`) null)
    (`|PlayMontage` (`/Game/aSuperHot/Blueprints/BP_PlayerCharacter.FirstPersonMesh` (`self.First PersonCharacter`)) "/Game/aSuperHot/Animation/AM_FiringRifle.AM_FiringRifle" 0.5
      (:`then`
        (`GameplayStatics.SetGlobalTimeDilation` 0.5)
        (`KismetSystemLibrary.Delay` 0.05)
        (`GameplayStatics.SetGlobalTimeDilation` (`/Game/aSuperHot/Blueprints/BP_TimeDilationVariable.TimeDilationControl` (`self.TimeDilationVariable`)))
        (`/Engine/EditorBlueprintResources/StandardMacros.DoOnce` false
          (:`Completed`
            (bind _outactors (`GameplayStatics.GetAllActorsOfClass` "/Game/aSuperHot/Blueprints/AI/BP_EnemyAIController.BP_EnemyAIController_C"))
            (for _array_element _outactors
              (`/Game/aSuperHot/Blueprints/AI/BP_EnemyAIController.OnPlayerAttackHeard` _array_element))))))))

(event `EnhancedInput|/Game/aSuperHot/Input/Actions/IA_Throw`
  (params (ActionValue :type Boolean) (ElapsedSeconds :type "Float (double-precision)") (TriggeredSeconds :type "Float (double-precision)") (InputAction :type "InputAction Object Reference" :default "/Game/aSuperHot/Input/Actions/IA_Throw.IA_Throw"))
  (bind _returnvalue (`PlayerCameraManager.GetCameraRotation` (`GameplayStatics.GetPlayerCameraManager` 0)))
  (:`Triggered`
    (`|PlayMontage` (`/Game/aSuperHot/Blueprints/BP_PlayerCharacter.FirstPersonMesh` (`self.First PersonCharacter`)) "/Game/aSuperHot/Animation/AM_Throwing.AM_Throwing"
      (:`then`
        (`|SpawnActorFromClass` "/Game/aSuperHot/Blueprints/Projectile/BP_RifleProjectile.BP_RifleProjectile_C" (`KismetMathLibrary.MakeTransform` (+ (`self.GetSocketLocation` "ThrowTransform") (`KismetMathLibrary.GreaterGreater_VectorRotator` (`self.ProjectileOffset`) _returnvalue)) _returnvalue) "Undefined" "OverrideRootScale" (`self.GetOwner`) null)
        (`/Game/aSuperHot/Blueprints/BP_PlayerCharacter.IsEquipWeapon` (`self.First PersonCharacter`))
        (`/Engine/EditorBlueprintResources/StandardMacros.DoOnce` false
          (:`Completed`
            (bind _outactors (`GameplayStatics.GetAllActorsOfClass` "/Game/aSuperHot/Blueprints/AI/BP_EnemyAIController.BP_EnemyAIController_C"))
            (for _array_element _outactors
              (`/Game/aSuperHot/Blueprints/AI/BP_EnemyAIController.OnPlayerAttackHeard` _array_element))))))))